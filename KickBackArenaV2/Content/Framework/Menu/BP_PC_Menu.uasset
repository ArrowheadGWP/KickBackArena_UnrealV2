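; Player controller for the menu and multiplayer lobby that gives the local player cursor and UI-only input.
; Initial setup loads the saved profile, creating a save slot if none exists, and passes it through ServerUpdateLobby to BP_GMB_Menu to refresh the lobby.
; It also creates and shows the lobby widget and updates its player names.
; Ending a client session destroys it and, on success, opens MainMenu.
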(event Custom|EndClientSession
  (|DestroySession self
    (:OnSuccess
      (Game|OpenLevel(byName) "MainMenu"))))

(event Custom|CreateLobbyMenu
  (CallFunction|UIShowLobbyMenu))

(event Custom|InitialSetup
  (CallFunction|LoadSavedProfile)
  (CallFunction|ServerUpdateLobby (Variables|Default|GetPlayer%20Profile%20Info)))

(event Custom|UpdatePlayerNames
  (params (PlayerProfiles :type Array%20of%20S%20Player%20Profile%20Structures))
  (bind _wbp_lobbymenu (Variables|Default|GetWBP_LobbyMenu))
  (Utilities|IsValid _wbp_lobbymenu
    (:Is%20Valid
      (Default|ClearPlayerNames _wbp_lobbymenu)
      (Default|UpdatePlayerNames _wbp_lobbymenu PlayerProfiles))))

(event Custom|ServerUpdateLobby
  (params (PlayerProfile :type S%20Player%20Profile%20Structure))
  (Variables|Default|SetPlayer%20Profile%20Info PlayerProfile)
  (bind _asbp_gmb_menu (Utilities|Casting|CastToBP_GMB_Menu (Game|GetGameMode)))
  (Default|UpdateLobby _asbp_gmb_menu true))

(event EventBeginPlay
  (if (Pawn|IsLocalController)
    (Variables|Default|SetbShowMouseCursor true)
    (Input|SetInputModeUIOnly self 0 "DoNotLock" false)))

(fn ConstructionScript)

(fn UIShowLobbyMenu
  (Utilities|IsValid (Variables|Default|GetWBP_LobbyMenu)
    (:Is%20Valid
      _)
    (:Is%20Not%20Valid
      (bind _returnvalue (UserInterface|CreateWidget "/Game/Widgets/WBP_LobbyMenu.WBP_LobbyMenu_C" self))
      (Variables|Default|SetWBP_LobbyMenu _returnvalue)))
  (UserInterface|Viewport|AddtoViewport (Variables|Default|GetWBP_LobbyMenu) 0)
  (return))

(fn LoadSavedProfile
  (bind _returnvalue (SaveGame|DoesSaveGameExist (LocalVariables|GetLocalSlotName)))
  (if _returnvalue
    _
    (else
      (bind _returnvalue_2 (SaveGame|CreateSaveGameObject "/Game/SavedData/BP_SG_PlayerProfile.BP_SG_PlayerProfile_C"))
      (SaveGame|SaveGametoSlot _returnvalue_2 (LocalVariables|GetLocalSlotName))))
  (bind _returnvalue_3 (SaveGame|LoadGamefromSlot (LocalVariables|GetLocalSlotName)))
  (bind _asbp_sg_player_profile (Utilities|Casting|CastToBP_SG_PlayerProfile _returnvalue_3))
  (Variables|Default|SetPlayer%20Profile%20Info (Variables|/Game/SavedData/BP_SG_PlayerProfile.BP_SG_PlayerProfile_C|GetPlayerProfile _asbp_sg_player_profile))
  (return))