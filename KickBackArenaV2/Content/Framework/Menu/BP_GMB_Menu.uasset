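; Menu game mode that manages players joining the lobby and keeps their profile lists in sync.
; When a new player starts in the Lobby Menu level, it registers their BP_PC_Menu controller, then triggers lobby menu creation and initial setup on it.
; UpdateLobby, when flagged for player names, rebuilds the profile list from all registered controllers and pushes it back to each one.
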(event Custom|UpdateLobby
  (params (PlayerNames :type Boolean))
  (if PlayerNames
    (Utilities|Array|Clear (Variables|Default|GetPlayerProfiles_All))
    (for _array_element (Variables|Default|GetAllConnectedPlayers)
      (Utilities|Array|Add (Variables|Default|GetPlayerProfiles_All) (Variables|/Game/Framework/Menu/BP_PC_Menu.BP_PC_Menu_C|GetPlayer%20Profile%20Info _array_element)))
    (for _array_element_2 (Variables|Default|GetAllConnectedPlayers)
      (if PlayerNames
        (Default|UpdatePlayerNames _array_element_2 (Variables|Default|GetPlayerProfiles_All))))))

(event EventBeginPlay)

(event EventTick
  (params (DeltaSeconds :type Float%20%28single-precision%29)))

(event EventHandleStartingNewPlayer
  (params (NewPlayer :type Player%20Controller%20Object%20Reference))
  (bind _returnvalue (Game|GetCurrentLevelName true))
  (switch string _returnvalue
    (:LobbyMenu
      (bind _asbp_pc_menu (Utilities|Casting|CastToBP_PC_Menu NewPlayer))
      (Utilities|Array|Add (Variables|Default|GetAllConnectedPlayers) _asbp_pc_menu)
      (Default|CreateLobbyMenu _asbp_pc_menu)
      (Default|InitialSetup _asbp_pc_menu))))

(fn ConstructionScript)