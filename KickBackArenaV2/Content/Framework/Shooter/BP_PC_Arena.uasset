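; BP_PC_Arena is the player controller for the shooter arena, owning the in-game HUD and the client's exit from a session.
; On BeginPlay the local controller clears existing widgets, creates or reuses WBP_InGameHUD and switches to game-only input without a cursor.
; Custom events re-enable pawn input, forward the start countdown to the HUD and unhide it.
; EndClientSession resets the GameInstance pause-menu flag, destroys the session, then opens MainMenu.
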(event Custom|EnableAllInputs
  (Input|EnableInput (Pawn|GetControlledPawn) self))

(event Custom|GameStartCoutdown
  (Default|GameStartCountdown (Variables|Default|GetWBP_InGameHUD)))

(event Custom|Unhide_IngameHUD
  (Widget|SetVisibility (Variables|Default|GetWBP_InGameHUD) "Visible"))

(event Custom|EndClientSession
  (bind _asbp_gi_arena_menu (Utilities|Casting|CastToBP_GI_ArenaMenu (Game|GetGameInstance)))
  (Variables|/Game/Framework/Menu/BP_GI_ArenaMenu.BP_GI_ArenaMenu_C|SetMulti_IsPauseMenuVisabile _asbp_gi_arena_menu false)
  (|DestroySession self
    (:then
      (Game|OpenLevel(byName) "MainMenu"))))

(event EventBeginPlay
  (if (Pawn|IsLocalPlayerController)
    (Viewport|RemoveAllWidgets)
    (CallFunction|UIShowinGameHUD)
    (Input|SetInputModeGameOnly self false)
    (Variables|Default|SetbShowMouseCursor false)))

(fn ConstructionScript)

(fn UIShowinGameHUD
  (Utilities|IsValid (Variables|Default|GetWBP_InGameHUD)
    (:Is%20Valid
      _)
    (:Is%20Not%20Valid
      (bind _returnvalue (UserInterface|CreateWidget "/Game/Widgets/WBP_InGameHUD.WBP_InGameHUD_C" self))
      (Variables|Default|SetWBP_InGameHUD _returnvalue)))
  (UserInterface|Viewport|AddtoViewport (Variables|Default|GetWBP_InGameHUD) 0)
  (return))