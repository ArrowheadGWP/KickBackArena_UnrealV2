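; Game mode for the Shooter arena that holds back spawning until the expected players join, then starts the match with a countdown.
; It collects arena player controllers and reads the connected-player count and solo flag from the arena menu game instance.
; Solo games spawn immediately; otherwise, once all have joined, each player spawns at the PlayerStart tagged with their join index.
; LevelStart then triggers each controller's countdown and enables input after a fixed delay.
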(event Custom|LevelStart
  (Utilities|FlowControl|Delay 0.2)
  (for _array_element (Variables|Default|GetAll_connectedControllers)
    (Default|GameStartCoutdown _array_element))
  (Utilities|FlowControl|Delay 3.0)
  (for _array_element_2 (Variables|Default|GetAll_connectedControllers)
    (Default|EnableAllInputs _array_element_2)))

(event EventHandleStartingNewPlayer
  (params (NewPlayer :type Player%20Controller%20Object%20Reference))
  ;[0.15 0.15 0.15 0.5] Starting new players
  (bind _asbp_pc_arena (Utilities|Casting|CastToBP_PC_Arena NewPlayer))
  (Utilities|Array|Add (Variables|Default|GetAll_connectedControllers) _asbp_pc_arena)
  (bind _asbp_gi_arena_menu (Utilities|Casting|CastToBP_GI_ArenaMenu (Game|GetGameInstance)))
  (Variables|Default|SetNumOfExepectedPlayers (Variables|/Game/Framework/Menu/BP_GI_ArenaMenu.BP_GI_ArenaMenu_C|GetNum%20Connected%20Players _asbp_gi_arena_menu))
  (if (Variables|/Game/Framework/Menu/BP_GI_ArenaMenu.BP_GI_ArenaMenu_C|GetIsSoloGame _asbp_gi_arena_menu)
    (Variables|Default|SetNumOfExepectedPlayers 1)
    (Class|GameModeBase|RestartPlayeratPlayerStart (Utilities|Array|Get(acopy) (Variables|Default|GetAll_connectedControllers)) (Class|GameModeBase|FindPlayerStart 0 "0"))
    (CallFunction|LevelStart)
    (elif (== (Variables|Default|GetNumOfExepectedPlayers) (Utilities|Array|Length (Variables|Default|GetAll_connectedControllers)))
      (Utilities|FlowControl|Delay 0.5)
      (for (_array_element _array_index) (Variables|Default|GetAll_connectedControllers)
        (Class|GameModeBase|RestartPlayeratPlayerStart _array_element (Class|GameModeBase|FindPlayerStart _array_element (Utilities|String|ToString(Integer) _array_index))))
      (CallFunction|LevelStart))))

(fn ConstructionScript)